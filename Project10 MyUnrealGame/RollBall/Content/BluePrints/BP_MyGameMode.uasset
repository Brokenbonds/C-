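; BP_MyGameMode is a game mode that handles the end of a game with a win screen and restart or quit keys.
; It enables its own input on BeginPlay so it can receive key presses.
; The EndGame event disables input on the player's BP_Character, shows BP_WinScreen and sets a GameEnding flag.
; Once that flag is set, Q quits the game and R reopens Map2.
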(event Custom|EndGame
  (bind _asbp_character (Utilities|Casting|CastToBP_Character (Game|Player|GetPlayerPawn 0)))
  (Input|DisableInput _asbp_character (Game|GetPlayerController 0))
  (bind _returnvalue (UserInterface|CreateWidget "/Game/BluePrints/BP_WinScreen.BP_WinScreen_C"))
  (UserInterface|Viewport|AddtoPlayerScreen _returnvalue)
  (Variables|Default|SetGameEnding true))

(event EventBeginPlay
  (Input|EnableInput (Game|GetPlayerController 0)))

(event Input|KeyboardEvents|Q
  (params (Key :type Key%20Structure :default "None"))
  (:Pressed
    (if (Variables|Default|GetGameEnding)
      (Game|QuitGame 0 "Quit" false))))

(event Input|KeyboardEvents|R
  (params (Key :type Key%20Structure :default "None"))
  (:Pressed
    (if (Variables|Default|GetGameEnding)
      (Game|OpenLevel(byName) "Map2" false))))

(fn ConstructionScript)