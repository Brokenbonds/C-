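; BP_Finishline is the finish line actor that ends the game when the ball reaches it.
; When a BP_Ball begins overlapping its Box, it swaps the FinishLine material to a finished look, sets very high angular damping on the ball's Sphere, and calls EndGame on BP_MyGameMode.
; When the ball leaves the box, only the normal finish line material is restored.
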(event OnComponentBeginOverlap(Box)
  (params (OverlappedComponent :type Primitive%20Component%20Object%20Reference) (OtherActor :type Actor%20Object%20Reference) (OtherComp :type Primitive%20Component%20Object%20Reference) (OtherBodyIndex :type Integer) (bFromSweep :type Boolean) (SweepResult :type Hit%20Result%20Structure%20%28by%20ref%29))
  ;[1 1 1] Ball interaction
  (bind _asbp_ball (Utilities|Casting|CastToBP_Ball OtherActor))
  (Rendering|Material|SetMaterial (Variables|Default|GetFinishLine) 0 "/Game/Materials/N_FinishLineFinished.N_FinishLineFinished")
  (Class|PrimitiveComponent|SetAngularDamping (Variables|/Game/BluePrints/BP_Ball.BP_Ball_C|GetSphere _asbp_ball) 2e+03)
  (CallFunction|EndGame))

(event OnComponentEndOverlap(Box)
  (params (OverlappedComponent :type Primitive%20Component%20Object%20Reference) (OtherActor :type Actor%20Object%20Reference) (OtherComp :type Primitive%20Component%20Object%20Reference) (OtherBodyIndex :type Integer))
  ;[1 1 1] Ball interaction
  (Utilities|Casting|CastToBP_Ball OtherActor)
  (Rendering|Material|SetMaterial (Variables|Default|GetFinishLine) 0 "/Game/Materials/N_FinishLine.N_FinishLine"))

(event Custom|EndGame
  ;[1 1 1] Stop Player from moving
  (bind _asbp_my_game_mode (Utilities|Casting|CastToBP_MyGameMode (Game|GetGameMode)))
  (Default|EndGame _asbp_my_game_mode))

(event EventBeginPlay)

(event EventTick
  (params (DeltaSeconds :type Float%20%28single-precision%29)))

(fn ConstructionScript)